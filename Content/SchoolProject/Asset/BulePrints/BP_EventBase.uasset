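; BP_EventBase is a base Blueprint for game events whose completion status persists in BP_GameInstance.
; The construction script derives EventName from the object's display name to key the saved status.
; On BeginPlay it reads that status, reapplies SetEventFinished if already Finished, and otherwise saves it as Unfinished.
; SetEventFinished and SetRestart switch the status and write it back to the GameInstance.
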(event EventBeginPlay
  ;[0.15 0.15 0.15 0.5] 開始時自身が以前に使用されているなら使用済み処理を呼び出す
  (bind _asbp_game_instance (Utilities|Casting|CastToBP_GameInstance (Game|GetGameInstance)))
  (bind _output_get (Variables|Default|SetGameInstance _asbp_game_instance))
  (bind _output_get_2 (Variables|Default|SetEventStatus (Default|GetEventStatus _output_get (Variables|Default|GetEventName))))
  (switch Utilities|FlowControl|Switch|SwitchonEN_EventStatus _output_get_2
    (:NewEnumerator0
      (Default|SaveEventStatus (Variables|Default|GetGameInstance) (Variables|Default|GetEventName) "NewEnumerator1"))
    (:NewEnumerator2
      (CallFunction|SetEventFinished))))

(fn ConstructionScript
  ;[0.15 0.15 0.15 0.5] コンストラクタ
  (Variables|Default|SetEventName (Utilities|String|StringToName (Utilities|GetDisplayName self))))

(fn SetEventFinished
  ;[0.15 0.15 0.15 0.5] 使用時処理関数
  (bind _output_get (Variables|Default|SetEventStatus "NewEnumerator2"))
  (Default|SaveEventStatus (Variables|Default|GetGameInstance) (Variables|Default|GetEventName) _output_get))

(fn SetRestart
  ;[0.15 0.15 0.15 0.5] リセット関数
  (bind _output_get (Variables|Default|SetEventStatus "NewEnumerator1"))
  (Default|SaveEventStatus (Variables|Default|GetGameInstance) (Variables|Default|GetEventName) _output_get))