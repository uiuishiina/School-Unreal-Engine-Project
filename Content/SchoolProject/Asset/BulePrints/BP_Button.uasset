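; BP_Button is a pressable button that triggers once the player steps into its Box trigger.
; An overlap by BP_Player plays the PushButton timeline, which drives the STMButton component's relative Z to animate the press.
; When the timeline finishes, SetEventFinished calls the parent version, disables Box collision so it cannot be pressed again, and sets the button's final relative location.
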(event OnComponentBeginOverlap(Box)
  (params (OverlappedComponent :type Primitive%20Component%20Object%20Reference) (OtherActor :type Actor%20Object%20Reference) (OtherComp :type Primitive%20Component%20Object%20Reference) (OtherBodyIndex :type Integer) (bFromSweep :type Boolean) (SweepResult :type Hit%20Result%20Structure%20%28by%20ref%29))
  ;[0.15 0.15 0.15 0.5] Buttonが押された時の処理
  (Utilities|Casting|CastToBP_Player OtherActor)
  (bind _vectorz (Timeline|PushButton Play)
    (:Update
      (Transformation|SetRelativeLocation (Variables|Default|GetSTM_Button) (Math|Vector|MakeVector 0.0 0.0 _vectorz) false false))
    (:Finished
      (CallFunction|SetEventFinished))))

(event EventBeginPlay
  ;[0.15 0.15 0.15 0.5] OnStart
  (|CallParentFunction))

(fn ConstructionScript)

(fn SetEventFinished
  ;[0.15 0.15 0.15 0.5] 押されたとき当たり判定を消す関数
  (|CallParentFunction)
  (Collision|SetCollisionEnabled (Variables|Default|GetBox) "NoCollision")
  (Transformation|SetRelativeLocation (Variables|Default|GetSTM_Button) (Math|Vector|MakeVector 0.0 0.0 0.0) false false))